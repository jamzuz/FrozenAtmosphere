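; BP_Laser is a laser beam actor that damages whatever it strikes along its forward vector.
; Every Tick it line traces on the Camera channel out to Distance and applies fixed damage to the hit actor, with no cooldown or delta-time scaling.
; The Niagara beam's LaserEnd parameter follows the hit point or full trace end, and a separate impact effect moves there, visible only on blocking hits.
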(event `self.ReceiveTick`
  (params (DeltaSeconds :type "Float (single-precision)"))
  (bind _returnvalue (`self.K2_GetActorLocation`))
  (bind _returnvalue_2 (+ _returnvalue (* (`self.GetActorForwardVector`) (`self.Distance`))))
  (set `self.TraceEnd` _returnvalue_2)
  (bind _outhit (`KismetSystemLibrary.LineTraceSingle` :`Start` _returnvalue :`End` _returnvalue_2 :`TraceChannel` "TraceTypeQuery2" :`TraceColor` (struct :`G` 0.152722 :`B` 1.0 :`A` 1.0)))
  (bind (_bblockinghit _binitialoverlap _time _distance _location _impactpoint _normal _impactnormal _physmat _hitactor) (`GameplayStatics.BreakHitResult` _outhit))
  (set `self.Location` _location)
  (set `self.Blocking Hit` _bblockinghit)
  (`GameplayStatics.ApplyDamage` _hitactor 100.0)
  (`FXSystemComponent.SetVectorParameter` (`self.NiagaraLaser`) "LaserEnd" (select `bool` (`self.Blocking Hit`) :`false` (`self.TraceEnd`) :`true` (`self.Location`)))
  (`SceneComponent.SetVisibility` (`self.NiagaraLaserImpact`) (`self.Blocking Hit`) false)
  (`SceneComponent.K2_SetWorldLocation` (`self.NiagaraLaserImpact`) (`self.Location`) false false))

(fn `UserConstructionScript`)