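; Doorway actor that a power cell powers up so its child door can work.
; When a PowerCell first enters the sphere, its core mesh attaches to the socket cube, a confirm sound plays and the cell's Door function is called.
; After a short delay it flags the child door as powered, marks itself done and opens the door (Avaa) if the player is already inside the door's trigger.
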(event `self.Sphere.OnComponentBeginOverlap`
  (params (OverlappedComponent :type "PrimitiveComponent Object Reference") (OtherActor :type "Actor Object Reference") (OtherComp :type "PrimitiveComponent Object Reference") (OtherBodyIndex :type Integer) (bFromSweep :type Boolean) (SweepResult :type "HitResult Structure (by ref)"))
  (bind _cube (`self.Cube`))
  (if (not (`self.done`))
    (bind _aspower_cell (cast `/Game/JesseAssets/Blueprints/PowerCell` OtherActor))
    (`SceneComponent.K2_AttachToComponent` (`/Game/JesseAssets/Blueprints/PowerCell.SM_EnergyCore_A` _aspower_cell) _cube "None" "KeepRelative" "KeepRelative" "KeepWorld" true)
    (`|ExecutionSequence`
      (:`then_0`
        (`GameplayStatics.PlaySoundAtLocation` "/Game/Aanet/Ui-confirm.Ui-confirm" (`SceneComponent.K2_GetComponentLocation` _cube) (struct) 0.5 1.0 0.0 "/Game/Aanet/ovi.ovi" null null)
        (`KismetSystemLibrary.Delay` 0.3)
        (bind _asdoorwaydoor (cast `/Game/JesseAssets/Blueprints/Doorwaydoor` (`ChildActorComponent.ChildActor` (`self.Doorwaydoor`))))
        (set `/Game/JesseAssets/Blueprints/Doorwaydoor.POWERCELL` true _asdoorwaydoor)
        (set `self.done` true)
        (`/Engine/EditorBlueprintResources/StandardMacros.DoOnce` false
          (:`Completed`
            (if (`PrimitiveComponent.IsOverlappingActor` (`/Game/JesseAssets/Blueprints/Doorwaydoor.Trigger` _asdoorwaydoor) (`GameplayStatics.GetPlayerPawn` 0))
              (`/Game/JesseAssets/Blueprints/Doorwaydoor.avaa` _asdoorwaydoor)))))
      (:`then_1`
        (`/Game/JesseAssets/Blueprints/PowerCell.Door` _aspower_cell)))))

(fn `UserConstructionScript`)