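; PowerCell is an actor with a physics Cylinder and an energy core mesh, exposing events for door, charger and red-cell interactions.
; When the Cylinder's body wakes, it spawns a replacement PowerCell at the core's transform.
; Door destroys the Cylinder, while Charger destroys both Cylinder and core.
; RedCell spawns a RedPowerCell at the core, puts its body to sleep, then runs Charger; every event fires only once.
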(event `Door`
  (`/Engine/EditorBlueprintResources/StandardMacros.DoOnce` false
    (:`Completed`
      (`ActorComponent.K2_DestroyComponent` (`self.Cylinder`)))))

(event `Charger`
  (`/Engine/EditorBlueprintResources/StandardMacros.DoOnce` false
    (:`Completed`
      (`|ExecutionSequence`
        (:`then_0`
          (`ActorComponent.K2_DestroyComponent` (`self.Cylinder`)))
        (:`then_1`
          (`ActorComponent.K2_DestroyComponent` (`self.SM_EnergyCore_A`)))))))

(event `RedCell`
  (`/Engine/EditorBlueprintResources/StandardMacros.DoOnce` false
    (:`Completed`
      (bind _returnvalue (`|SpawnActorFromClass` "/Game/JesseAssets/Blueprints/RedPowerCell.RedPowerCell_C" (`SceneComponent.K2_GetComponentToWorld` (`self.SM_EnergyCore_A`)) "AlwaysSpawn" "OverrideRootScale" null null))
      (`PrimitiveComponent.PutRigidBodyToSleep` (`/Game/JesseAssets/Blueprints/RedPowerCell.Cylinder` _returnvalue) "None")
      (`self.Charger`))))

(event `self.Cylinder.OnComponentWake`
  (params (WakingComponent :type "PrimitiveComponent Object Reference") (BoneName :type Name))
  (`/Engine/EditorBlueprintResources/StandardMacros.DoOnce` false
    (:`Completed`
      (`|SpawnActorFromClass` "PowerCell_C" (`SceneComponent.K2_GetComponentToWorld` (`self.SM_EnergyCore_A`)) "AlwaysSpawn" "OverrideRootScale" null null))))

(fn `UserConstructionScript`)