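; Fuse puzzle socket that accepts a greencell actor overlapping its Overlap component.
; It gets rid of the incoming cell, spawns a fresh one snapped to Greencube, wakes it, fires the Fusepuzzleplus dispatcher and plays a confirm sound.
; A DoOnce guards the swap and resets right after it.
; When the stored spawned cell leaves the overlap, the socket fires Fusepuzzleminus.
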(event `self.overlap.OnComponentBeginOverlap`
  (params (OverlappedComponent :type "PrimitiveComponent Object Reference") (OtherActor :type "Actor Object Reference") (OtherComp :type "PrimitiveComponent Object Reference") (OtherBodyIndex :type Integer) (bFromSweep :type Boolean) (SweepResult :type "HitResult Structure (by ref)"))
  (bind _asgreencell (cast `/Game/JesseAssets/Blueprints/greencell` OtherActor))
  (`/Engine/EditorBlueprintResources/StandardMacros.DoOnce` false :!label _label
    (:`Completed`
      (`self.fuseitup`))))

(event `fuseitup`
  (bind _greencube (`self.greencube`))
  (`/Game/JesseAssets/Blueprints/greencell.getridofit` (stale `self.overlap.OnComponentBeginOverlap` _asgreencell))
  (bind _returnvalue (`|SpawnActorFromClass` "/Game/JesseAssets/Blueprints/greencell.greencell_C" (`KismetMathLibrary.MakeTransform` (0.0 0.0 0.0)) "Undefined" "OverrideRootScale" null null))
  (`|ExecutionSequence`
    (:`then_0`
      (`self.K2_AttachToComponent` _returnvalue _greencube "None" "SnapToTarget" "SnapToTarget" "KeepWorld" true)
      (`/Game/JesseAssets/Blueprints/greencell.wakeupidiot` _returnvalue)
      (`self.fusepuzzleplus`)
      (`GameplayStatics.PlaySoundAtLocation` "/Game/Aanet/Ui-confirm.Ui-confirm" (`SceneComponent.K2_GetComponentLocation` _greencube) (struct) 0.6 1.0 0.0 "/Game/JesseAssets/aanet/laseratten.laseratten" null null)
      (goto _label :!via `Reset`))
    (:`then_1`
      (set `self.SpawnedObject` _returnvalue))))

(event `self.overlap.OnComponentEndOverlap`
  (params (OverlappedComponent :type "PrimitiveComponent Object Reference") (OtherActor :type "Actor Object Reference") (OtherComp :type "PrimitiveComponent Object Reference") (OtherBodyIndex :type Integer))
  (if (== OtherActor (`self.SpawnedObject`))
    (`self.fusepuzzleminus`)))

(fn `UserConstructionScript`)