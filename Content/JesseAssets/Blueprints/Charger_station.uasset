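; Charger station Blueprint that docks a PowerCell entering its Sphere trigger and switches it to its red state.
; On overlap, it disables physics on the cell's core and yellow cylinder meshes, then attaches the core mesh to the station's Cube with welding.
; A confirm sound plays at the Cube, followed one second later by a deny sound and the cell's RedCell call.
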(event `self.Sphere.OnComponentBeginOverlap`
  (params (OverlappedComponent :type "PrimitiveComponent Object Reference") (OtherActor :type "Actor Object Reference") (OtherComp :type "PrimitiveComponent Object Reference") (OtherBodyIndex :type Integer) (bFromSweep :type Boolean) (SweepResult :type "HitResult Structure (by ref)"))
  (bind _cube (`self.Cube`))
  (bind _returnvalue (`SceneComponent.K2_GetComponentLocation` _cube))
  (bind _aspower_cell (cast `/Game/JesseAssets/Blueprints/PowerCell` OtherActor))
  (bind _sm_energycore_a (`/Game/JesseAssets/Blueprints/PowerCell.SM_EnergyCore_A` _aspower_cell))
  (`PrimitiveComponent.SetSimulatePhysics` _sm_energycore_a false)
  (`PrimitiveComponent.SetSimulatePhysics` (`/Game/JesseAssets/Blueprints/PowerCell.Cylinder(yellow)` _aspower_cell) false)
  (`SceneComponent.K2_AttachToComponent` _sm_energycore_a _cube "None" "KeepRelative" "KeepRelative" "KeepWorld" true)
  (`GameplayStatics.PlaySoundAtLocation` "/Game/Aanet/Ui-confirm.Ui-confirm" _returnvalue (struct) 0.5 1.0 0.0 "/Game/Aanet/ovi.ovi" null null)
  (`KismetSystemLibrary.Delay` 1.0)
  (`GameplayStatics.PlaySoundAtLocation` "/Game/Aanet/Ui-deny.Ui-deny" _returnvalue (struct) 0.5 1.0 0.0 "/Game/Aanet/ovi.ovi" null null)
  (`/Game/JesseAssets/Blueprints/PowerCell.RedCell` _aspower_cell))

(fn `UserConstructionScript`)