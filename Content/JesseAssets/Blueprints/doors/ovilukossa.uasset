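; A locked sliding door Blueprint that opens for the first-person character only when its Puzzledone flag is set.
; Entering the trigger either plays a deny sound or activates two steam effects, plays confirm and hiss sounds, and runs a timeline.
; The timeline lerps the door mesh between closed and open relative locations, reversing when the character leaves the trigger.
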(event `self.Trigger.OnComponentBeginOverlap`
  (params (OverlappedComponent :type "PrimitiveComponent Object Reference") (OtherActor :type "Actor Object Reference") (OtherComp :type "PrimitiveComponent Object Reference") (OtherBodyIndex :type Integer) (bFromSweep :type Boolean) (SweepResult :type "HitResult Structure (by ref)"))
  (bind _returnvalue (`SceneComponent.K2_GetComponentLocation` (`self.Door_Small_A`)))
  (cast `/Game/FirstPersonBP/Blueprints/FirstPersonCharacter` OtherActor)
  (if (`self.puzzledone`)
    (`ActorComponent.Activate` (`self.SteamDoor`) false)
    (`ActorComponent.Activate` (`self.SteamDoor2`) false)
    (`GameplayStatics.PlaySoundAtLocation` "/Game/Aanet/Ui-confirm.Ui-confirm" _returnvalue (struct) 0.3 1.0 0.0 "/Game/Aanet/ovi.ovi" null null)
    (`GameplayStatics.PlaySoundAtLocation` "/Game/Aanet/hiss_door.hiss_door" _returnvalue (struct) 0.2 1.0 0.0 "/Game/Aanet/ovi.ovi" null null)
    (bind (_direction _doorposition) (`Timeline|Timeline_0` :!label _label)
      (:`Update`
        (`SceneComponent.K2_SetRelativeLocation` (`self.Door_Small_A`) (`KismetMathLibrary.VLerp` (`self.DoorClosed`) (`self.DoorOpen`) _doorposition) false false)))
    (else
      (`GameplayStatics.PlaySoundAtLocation` "/Game/Aanet/Ui-deny.Ui-deny" (`SceneComponent.K2_GetComponentLocation` (`self.Door_Small_A`)) (struct) 0.3 1.0 0.0 "/Game/Aanet/ovi.ovi" null null))))

(event `self.Trigger.OnComponentEndOverlap`
  (params (OverlappedComponent :type "PrimitiveComponent Object Reference") (OtherActor :type "Actor Object Reference") (OtherComp :type "PrimitiveComponent Object Reference") (OtherBodyIndex :type Integer))
  (cast `/Game/FirstPersonBP/Blueprints/FirstPersonCharacter` OtherActor)
  (if (`self.puzzledone`)
    (goto _label :!via `Reverse`)))

(fn `UserConstructionScript`)