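; Door2 is a double sliding glass door that opens when the first-person character enters its Box trigger and closes when the character leaves.
; Overlap begin plays two timelines and overlap end reverses them.
; One timeline sets SMGlassDoorA's full relative location, while the other changes only the X of SMGlassDoorA1, keeping its Y and Z.
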(event `self.Box.OnComponentBeginOverlap`
  (params (OverlappedComponent :type "PrimitiveComponent Object Reference") (OtherActor :type "Actor Object Reference") (OtherComp :type "PrimitiveComponent Object Reference") (OtherBodyIndex :type Integer) (bFromSweep :type Boolean) (SweepResult :type "HitResult Structure (by ref)"))
  (bind _sm_glassdoor_a1 (`self.SM_GlassDoor_A1`))
  (cast `/Game/FirstPersonBP/Blueprints/FirstPersonCharacter` OtherActor)
  (`|ExecutionSequence`
    (:`then_0`
      (bind (_direction _newtrack_1) (`Timeline|Timeline_0` :!label _label)
        (:`Update`
          (`SceneComponent.K2_SetRelativeLocation` (`self.SM_GlassDoor_A`) _newtrack_1 false false))))
    (:`then_1`
      (bind (_direction_2 _newtrack_1_2) (`Timeline|Timeline_1` :!label _label_2)
        (:`Update`
          (`SceneComponent.K2_SetRelativeLocation` _sm_glassdoor_a1 (`KismetMathLibrary.MakeVector` (.x _newtrack_1_2) (.y (`SceneComponent.RelativeLocation` _sm_glassdoor_a1)) (.z (`SceneComponent.RelativeLocation` _sm_glassdoor_a1))) false false))))))

(event `self.Box.OnComponentEndOverlap`
  (params (OverlappedComponent :type "PrimitiveComponent Object Reference") (OtherActor :type "Actor Object Reference") (OtherComp :type "PrimitiveComponent Object Reference") (OtherBodyIndex :type Integer))
  (cast `/Game/FirstPersonBP/Blueprints/FirstPersonCharacter` OtherActor)
  (`|ExecutionSequence`
    (:`then_0`
      (goto _label :!via `Reverse`))
    (:`then_1`
      (goto _label_2 :!via `Reverse`))))

(fn `UserConstructionScript`)