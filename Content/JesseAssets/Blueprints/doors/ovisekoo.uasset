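; A door Blueprint that moves its left door mesh vertically and damages a first-person character that enters its box trigger.
; On BeginPlay, a timeline drives the mesh's relative Z without sweep.
; Each timeline update also spawns a quiet attenuated sound, using the doorway mesh's relative location as the world position.
; Box overlap applies heavy damage to the character, independent of the door's position.
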(event `self.ReceiveBeginPlay`
  (bind _sm_door_l (`self.SM_Door_L`))
  (bind (_direction _newtrack_0) (`Timeline|Timeline_0`)
    (:`Update`
      (`GameplayStatics.SpawnSoundAtLocation` "/Game/Aanet/Ui-deny.Ui-deny" (`SceneComponent.RelativeLocation` (`self.SM_Doorway_L`)) (struct) 0.01 1.0 0.0 "/Game/Aanet/ovi.ovi" null)
      (`SceneComponent.K2_SetRelativeLocation` _sm_door_l (`KismetMathLibrary.MakeVector` (.x (`SceneComponent.RelativeLocation` _sm_door_l)) (.y (`SceneComponent.RelativeLocation` _sm_door_l)) _newtrack_0) false false))))

(event `self.Box.OnComponentBeginOverlap`
  (params (OverlappedComponent :type "PrimitiveComponent Object Reference") (OtherActor :type "Actor Object Reference") (OtherComp :type "PrimitiveComponent Object Reference") (OtherBodyIndex :type Integer) (bFromSweep :type Boolean) (SweepResult :type "HitResult Structure (by ref)"))
  (bind _asfirst_person_character (cast `/Game/FirstPersonBP/Blueprints/FirstPersonCharacter` OtherActor))
  (`GameplayStatics.ApplyDamage` _asfirst_person_character 200.0))

(fn `UserConstructionScript`)