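; Spinny is a hazard actor with a sci-fi crate mesh that moves and two boxes that damage the player.
; On BeginPlay a timeline lerps the crate's relative location between Start and End; despite the name, the graph applies no rotation.
; Either box deals 100 damage to an overlapping FirstPersonCharacter through that character's TakeDamage.
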(event `self.ReceiveBeginPlay`
  (bind (_direction _newtrack_0) (`Timeline|Timeline_0`)
    (:`Update`
      (`SceneComponent.K2_SetRelativeLocation` (`self.SM_Scifi_Crate`) (`KismetMathLibrary.VLerp` (`self.Start`) (`self.End`) _newtrack_0) false false))))

(event `self.Box.OnComponentBeginOverlap`
  (params (OverlappedComponent :type "PrimitiveComponent Object Reference") (OtherActor :type "Actor Object Reference") (OtherComp :type "PrimitiveComponent Object Reference") (OtherBodyIndex :type Integer) (bFromSweep :type Boolean) (SweepResult :type "HitResult Structure (by ref)"))
  (bind _asfirst_person_character (cast `/Game/FirstPersonBP/Blueprints/FirstPersonCharacter` OtherActor))
  (`/Game/FirstPersonBP/Blueprints/FirstPersonCharacter.TakeDamage` _asfirst_person_character 100.0))

(event `self.Box1.OnComponentBeginOverlap`
  (params (OverlappedComponent :type "PrimitiveComponent Object Reference") (OtherActor :type "Actor Object Reference") (OtherComp :type "PrimitiveComponent Object Reference") (OtherBodyIndex :type Integer) (bFromSweep :type Boolean) (SweepResult :type "HitResult Structure (by ref)"))
  (bind _asfirst_person_character (cast `/Game/FirstPersonBP/Blueprints/FirstPersonCharacter` OtherActor))
  (`/Game/FirstPersonBP/Blueprints/FirstPersonCharacter.TakeDamage` _asfirst_person_character 100.0))

(fn `UserConstructionScript`)