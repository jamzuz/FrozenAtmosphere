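; RedPowerCell is an explosive prop that blows up when hit after its physics body wakes, or when it takes any damage.
; Waking the Cylinder arms hit detonation after a short delay, while damage detonates it at the energy core mesh without that check.
; Each trigger has its own DoOnce and duplicated sequence: explosion effect and sound, full radial damage, then a brief delay before a radial force impulse and self-destruction.
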(event `self.Cylinder.OnComponentWake`
  (params (WakingComponent :type "PrimitiveComponent Object Reference") (BoneName :type Name))
  (`KismetSystemLibrary.Delay` 0.5)
  (set `self.iswoke` true))

(event `self.Cylinder.OnComponentHit`
  (params (HitComponent :type "PrimitiveComponent Object Reference") (OtherActor :type "Actor Object Reference") (OtherComp :type "PrimitiveComponent Object Reference") (NormalImpulse :type "Vector Structure") (Hit :type "HitResult Structure (by ref)"))
  (bind (_bblockinghit _binitialoverlap _time _distance _location _impactpoint) (`GameplayStatics.BreakHitResult` Hit))
  (if (`self.iswoke`)
    (`/Engine/EditorBlueprintResources/StandardMacros.DoOnce` false
      (:`Completed`
        (`GameplayStatics.SpawnEmitterAtLocation` "/Game/StarterContent/Particles/P_Explosion.P_Explosion" _impactpoint (struct) (2.0 2.0 2.0))
        (`GameplayStatics.SpawnSoundAtLocation` "/Game/Aanet/Explosion_01.Explosion_01" _impactpoint (struct) 1.0 1.0 0.0 "/Game/Aanet/expl.expl" null)
        (`GameplayStatics.ApplyRadialDamage` :`BaseDamage` 500.0 :`Origin` _location :`DamageRadius` 300.0 :`DamageTypeClass` "/Script/Engine.DamageType" :`DamageCauser` null :`InstigatedByController` null :`bDoFullDamage` true :`DamagePreventionChannel` "ECC_GameTraceChannel3")
        (`KismetSystemLibrary.Delay` 0.2)
        (`RadialForceComponent.FireImpulse` (`self.RadialForce`))
        (`self.K2_DestroyActor`)))))

(event `self.ReceiveAnyDamage`
  (params (Damage :type "Float (single-precision)") (DamageType :type "DamageType Object Reference") (InstigatedBy :type "Controller Object Reference") (DamageCauser :type "Actor Object Reference"))
  (bind _returnvalue (`SceneComponent.K2_GetComponentLocation` (`self.SM_EnergyCore_A`)))
  (`/Engine/EditorBlueprintResources/StandardMacros.DoOnce` false
    (:`Completed`
      (`GameplayStatics.SpawnEmitterAtLocation` "/Game/StarterContent/Particles/P_Explosion.P_Explosion" _returnvalue (struct) (2.0 2.0 2.0))
      (`GameplayStatics.SpawnSoundAtLocation` "/Game/Aanet/Explosion_01.Explosion_01" _returnvalue (struct) 1.0 1.0 0.0 "/Game/Aanet/expl.expl" null)
      (`GameplayStatics.ApplyRadialDamage` :`BaseDamage` 500.0 :`Origin` _returnvalue :`DamageRadius` 300.0 :`DamageTypeClass` "/Script/Engine.DamageType" :`DamageCauser` null :`InstigatedByController` null :`bDoFullDamage` true :`DamagePreventionChannel` "ECC_GameTraceChannel3")
      (`KismetSystemLibrary.Delay` 0.2)
      (`RadialForceComponent.FireImpulse` (`self.RadialForce`))
      (`self.K2_DestroyActor`))))

(fn `UserConstructionScript`)