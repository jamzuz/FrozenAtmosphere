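; Explosive-breakable door Blueprint that is destroyed by radial damage and plays a deny sound when the player walks into it.
; The first radial hit, gated by a DoOnce, destroys the glass, UI and trigger box components and fires a debug-print destroyed event.
; A damage threshold comparison exists but is unwired, so any radial damage breaks it.
; Overlap of the box by the FirstPersonCharacter plays the attenuated sound at the door UI's location.
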(event `destroyed`
  (`KismetSystemLibrary.PrintString` "Door destroyed"))

(event `self.ReceiveRadialDamage`
  (params (DamageReceived :type "Float (single-precision)") (DamageType :type "DamageType Object Reference") (Origin :type "Vector Structure") (HitInfo :type "HitResult Structure (by ref)") (InstigatedBy :type "Controller Object Reference") (DamageCauser :type "Actor Object Reference"))
  (`/Engine/EditorBlueprintResources/StandardMacros.DoOnce` false
    (:`Completed`
      (`KismetSystemLibrary.PrintString` (`KismetStringLibrary.Conv_DoubleToString` DamageReceived))
      (`ActorComponent.K2_DestroyComponent` (`self.Door_Small_A_Glass`))
      (`ActorComponent.K2_DestroyComponent` (`self.Door_Small_UI`))
      (`ActorComponent.K2_DestroyComponent` (`self.Box`))
      (`self.destroyed`))))

(event `self.Box.OnComponentBeginOverlap`
  (params (OverlappedComponent :type "PrimitiveComponent Object Reference") (OtherActor :type "Actor Object Reference") (OtherComp :type "PrimitiveComponent Object Reference") (OtherBodyIndex :type Integer) (bFromSweep :type Boolean) (SweepResult :type "HitResult Structure (by ref)"))
  (cast `/Game/FirstPersonBP/Blueprints/FirstPersonCharacter` OtherActor)
  (`GameplayStatics.PlaySoundAtLocation` "/Game/Aanet/Ui-deny.Ui-deny" (`SceneComponent.K2_GetComponentLocation` (`self.Door_Small_UI`)) (struct) 1.0 1.0 0.0 "/Game/Aanet/ovi.ovi" null null))

(fn `UserConstructionScript`)