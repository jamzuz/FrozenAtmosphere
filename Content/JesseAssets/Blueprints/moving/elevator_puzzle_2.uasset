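; Elevator actor for a puzzle that, when the first-person character overlaps it, alternates after a short delay between raising and lowering.
; A FlipFlop plays or reverses a timeline that lerps the Arrow component's height, with beep and machine activation.
; On timeline finish, lights toggle and a one-time event detaches the attached child Vent and briefly wakes its grate's physics.
; The puzzle-done check with its deny sound is unconnected.
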(event `perilla`
  ;[1 1 1] enable the grate
  (`/Engine/EditorBlueprintResources/StandardMacros.DoOnce` false
    (:`Completed`
      (bind _asvent (cast `/Game/JesseAssets/Blueprints/Vent` (`ChildActorComponent.ChildActor` (`self.Vent`))))
      (bind _grate (`/Game/JesseAssets/Blueprints/Vent.grate` _asvent))
      (`PrimitiveComponent.SetSimulatePhysics` _grate true)
      (`SceneComponent.K2_DetachFromComponent` (`Actor.RootComponent` _asvent) "KeepRelative" "KeepRelative" "KeepRelative" true)
      (`KismetSystemLibrary.Delay` 0.2)
      (`PrimitiveComponent.PutRigidBodyToSleep` _grate "None"))))

(event `self.ReceiveBeginPlay`
  ;[1 1 1] disable grate
  (bind _asvent (cast `/Game/JesseAssets/Blueprints/Vent` (`ChildActorComponent.ChildActor` (`self.Vent`))))
  (`PrimitiveComponent.SetSimulatePhysics` (`/Game/JesseAssets/Blueprints/Vent.grate` _asvent) false)
  (`self.K2_AttachToComponent` _asvent (`self.hissi`) "None" "KeepWorld" "KeepWorld" "KeepWorld" true))

(event `self.ReceiveActorBeginOverlap`
  (params (OtherActor :type "Actor Object Reference"))
  ;[1 1 1] check if puzzle is done, continue accordingly
  (cast `/Game/FirstPersonBP/Blueprints/FirstPersonCharacter` OtherActor)
  (`KismetSystemLibrary.Delay` 1.5)
  (`/Engine/EditorBlueprintResources/StandardMacros.FlipFlop`
    (:`A`
      ;[1 1 1] go up
      (`GameplayStatics.PlaySoundAtLocation` "/Game/Aanet/Ui-confirm.Ui-confirm" (`SceneComponent.RelativeLocation` (`self.beep`)) (struct) 1.0 1.0 0.0 null null null)
      (`ActorComponent.Activate` (`self.machine`) true)
      ;[1 1 1] Change value to change height of elevator
      (bind (_direction _alpha) (`Timeline|Timeline_0` :!label _label)
        (:`Update`
          ;[1 1 1] Change Z of elevator and move it
          (`SceneComponent.K2_SetRelativeLocation` (`self.Arrow`) (`KismetMathLibrary.MakeVector` (.x (`SceneComponent.RelativeLocation` (`self.Arrow`))) (.y (`SceneComponent.RelativeLocation` (`self.Arrow`))) (.z (`KismetMathLibrary.VLerp` (`self.start`) (`self.end`) _alpha))) false false))
        (:`Finished`
          ;[1 1 1] send event to wake up grate
          (`self.perilla`)
          (`ActorComponent.Deactivate` (`self.machine`))
          (`SceneComponent.ToggleVisibility` (`self.SM_Light_B`) false)
          (`SceneComponent.ToggleVisibility` (`self.light off`) false)
          (`SceneComponent.ToggleVisibility` (`self.PointLight`) false)
          (`KismetSystemLibrary.Delay` 0.5)
          (`GameplayStatics.PlaySoundAtLocation` "/Game/Aanet/Fuze-switch.Fuze-switch" (`SceneComponent.K2_GetComponentLocation` (`self.PointLight1`)) (struct) 0.3 1.0 0.4 "/Game/Aanet/ovi.ovi" null null)
          (`KismetSystemLibrary.Delay` 0.5)
          (`SceneComponent.ToggleVisibility` (`self.PointLight1`) false))))
    (:`B`
      ;[1 1 1] go back
      (`GameplayStatics.PlaySoundAtLocation` "/Game/Aanet/Ui-confirm.Ui-confirm" (`SceneComponent.RelativeLocation` (`self.beep`)) (struct) 1.0 1.0 0.0 null null null)
      (`KismetSystemLibrary.Delay` 0.5)
      (`ActorComponent.Activate` (`self.machine`) true)
      (goto _label :!via `Reverse`))))

(fn `UserConstructionScript`)