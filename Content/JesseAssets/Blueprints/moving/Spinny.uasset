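; Spinny is a moving sci-fi crate hazard that deals heavy damage to the first-person character.
; On BeginPlay, the Package timeline slides the crate's relative location between Start and End without sweeping, despite the asset's name suggesting rotation.
; Each timeline update also sets the actor's custom time dilation from a slowness variable to control its pace.
; Overlapping the Box component applies the damage only to FirstPersonCharacter actors.
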(event `self.ReceiveBeginPlay`
  (bind (_direction _newtrack_0) (`Timeline|package`)
    (:`Update`
      (set `self.CustomTimeDilation` (`self.Howslow(0.1-1)`))
      (`SceneComponent.K2_SetRelativeLocation` (`self.SM_Scifi_Crate`) (`KismetMathLibrary.VLerp` (`self.Start`) (`self.End`) _newtrack_0) false false))))

(event `self.Box.OnComponentBeginOverlap`
  (params (OverlappedComponent :type "PrimitiveComponent Object Reference") (OtherActor :type "Actor Object Reference") (OtherComp :type "PrimitiveComponent Object Reference") (OtherBodyIndex :type Integer) (bFromSweep :type Boolean) (SweepResult :type "HitResult Structure (by ref)"))
  (bind _asfirst_person_character (cast `/Game/FirstPersonBP/Blueprints/FirstPersonCharacter` OtherActor))
  (`GameplayStatics.ApplyDamage` _asfirst_person_character 120.0 null null "/Script/Engine.DamageType"))

(fn `UserConstructionScript`)