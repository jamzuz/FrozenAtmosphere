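; Drawbridge actor that moves when a PowerCable enters its OverlapSilta trigger.
; The overlap plays the Down timeline, which drives the pitch of DrawbridgeMerge while showing the spotlight and setting the Greentored light to green.
; The same overlap snaps both of the cable's socket components onto Box2, plugging it in.
; The graph has no logic to reverse the bridge or detach the cable.
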(event `self.Overlap(silta).OnComponentBeginOverlap`
  (params (OverlappedComponent :type "PrimitiveComponent Object Reference") (OtherActor :type "Actor Object Reference") (OtherComp :type "PrimitiveComponent Object Reference") (OtherBodyIndex :type Integer) (bFromSweep :type Boolean) (SweepResult :type "HitResult Structure (by ref)"))
  (bind _aspower_cable (cast `/Game/JesseAssets/Blueprints/PowerCable` OtherActor))
  (`|ExecutionSequence`
    (:`then_0`
      (bind (_direction _newtrack_0) (`Timeline|down`)
        (:`Update`
          (`SceneComponent.K2_SetRelativeRotation` (`self.Drawbridge_merge`) (`KismetMathLibrary.MakeRotator` 0.0 _newtrack_0) false false)
          (`SceneComponent.SetVisibility` (`self.SpotLight`) true false)
          (`LightComponent.SetLightColor` (`self.greentored`) (struct :`G` 0.630208 :`B` 0.127487 :`A` 1.0) false))))
    (:`then_1`
      (`SceneComponent.K2_AttachToComponent` (`/Game/JesseAssets/Blueprints/PowerCable.Socket` _aspower_cable) (`self.box2`) "None" "SnapToTarget" "SnapToTarget" "SnapToTarget" true))
    (:`then_2`
      (`SceneComponent.K2_AttachToComponent` (`/Game/JesseAssets/Blueprints/PowerCable.Socket1` _aspower_cable) (`self.box2`) "None" "SnapToTarget" "SnapToTarget" "SnapToTarget" true))))

(fn `UserConstructionScript`)