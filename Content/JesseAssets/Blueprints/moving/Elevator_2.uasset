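; Elevator Blueprint that raises or lowers a sci-fi floor mesh while the first-person character is inside its trigger box.
; Box overlap plays a timeline after a short delay, lerping only the floor's relative Z between Start and End.
; Leaving the box reverses the timeline after a longer delay.
; The Machine component activates on each move and deactivates when the timeline finishes.
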(event `self.Box.OnComponentBeginOverlap`
  (params (OverlappedComponent :type "PrimitiveComponent Object Reference") (OtherActor :type "Actor Object Reference") (OtherComp :type "PrimitiveComponent Object Reference") (OtherBodyIndex :type Integer) (bFromSweep :type Boolean) (SweepResult :type "HitResult Structure (by ref)"))
  (bind _sm_scifi_floor_02 (`self.SM_Scifi_Floor_02`))
  (bind _machine (`self.machine`))
  ;[1 1 1] rinse and repeat
  (cast `/Game/FirstPersonBP/Blueprints/FirstPersonCharacter` OtherActor)
  (`KismetSystemLibrary.Delay` 0.5)
  (`|ExecutionSequence`
    (:`then_0`
      ;[1 1 1] Change value to change height of elevator
      (bind (_direction _alpha) (`Timeline|Timeline_0` :!label _label)
        (:`Update`
          ;[1 1 1] Change Z of elevator and move it
          (`SceneComponent.K2_SetRelativeLocation` _sm_scifi_floor_02 (`KismetMathLibrary.MakeVector` (.x (`SceneComponent.RelativeLocation` _sm_scifi_floor_02)) (.y (`SceneComponent.RelativeLocation` _sm_scifi_floor_02)) (.z (`KismetMathLibrary.VLerp` (`self.start`) (`self.end`) _alpha))) false false))
        (:`Finished`
          (`ActorComponent.Deactivate` _machine))))
    (:`then_1`
      (`ActorComponent.Activate` _machine true :!label _label_2))))

(event `self.Box.OnComponentEndOverlap`
  (params (OverlappedComponent :type "PrimitiveComponent Object Reference") (OtherActor :type "Actor Object Reference") (OtherComp :type "PrimitiveComponent Object Reference") (OtherBodyIndex :type Integer))
  (cast `/Game/FirstPersonBP/Blueprints/FirstPersonCharacter` OtherActor)
  (`KismetSystemLibrary.Delay` 2.0)
  (`|ExecutionSequence`
    (:`then_0`
      (goto _label :!via `Reverse`))
    (:`then_1`
      (goto _label_2))))

(fn `UserConstructionScript`)