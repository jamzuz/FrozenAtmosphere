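; Elevator actor that rises or descends between Start and End heights when the first-person character enters its Box trigger.
; Overlap plays a confirm sound, waits 1.5 seconds, then plays a timeline that lerps only Z and moves the actor without sweeping.
; Elevator and music cues attach to the Cube during travel and stop when the timeline finishes.
; The graph contains no return trip.
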(event `self.Box.OnComponentBeginOverlap`
  (params (OverlappedComponent :type "PrimitiveComponent Object Reference") (OtherActor :type "Actor Object Reference") (OtherComp :type "PrimitiveComponent Object Reference") (OtherBodyIndex :type Integer) (bFromSweep :type Boolean) (SweepResult :type "HitResult Structure (by ref)"))
  (bind _cube (`self.Cube`))
  ;[1 1 1] rinse and repeat
  (cast `/Game/FirstPersonBP/Blueprints/FirstPersonCharacter` OtherActor)
  (`GameplayStatics.PlaySoundAtLocation` "/Game/Aanet/Ui-confirm.Ui-confirm" (`SceneComponent.K2_GetComponentLocation` (`self.Elevator_00`)) (struct) 0.4 1.0 0.0 "/Game/Aanet/ovi.ovi" null null)
  (`KismetSystemLibrary.Delay` 1.5)
  ;[1 1 1] Chamge value to change height of elevator
  (`|ExecutionSequence`
    (:`then_0`
      (bind (_direction _height) (`Timeline|Timeline_0`)
        (:`Update`
          ;[1 1 1] Change Z of elevator and move it
          (`self.K2_SetActorRelativeLocation` (`KismetMathLibrary.MakeVector` (.x (`SceneComponent.RelativeLocation` (`self.Elevator_00`))) (.y (`SceneComponent.RelativeLocation` (`self.Elevator_00`))) (.z (`KismetMathLibrary.VLerp` (`self.start`) (`self.End`) _height)))))
        (:`Finished`
          (`AudioComponent.Stop` (stale _returnvalue))
          (`AudioComponent.Stop` (stale _returnvalue_2)))))
    (:`then_1`
      (bind _returnvalue (`GameplayStatics.SpawnSoundAttached` "/Game/JesseAssets/aanet/elevator_cue.elevator_cue" _cube "None" (0.0 0.0 0.0) (struct) "KeepRelativeOffset" false 1.0 1.0 0.0 null null))
      (bind _returnvalue_2 (`GameplayStatics.SpawnSoundAttached` "/Game/JesseAssets/aanet/ElevatorMusic_Cue.ElevatorMusic_Cue" _cube "None" (0.0 0.0 0.0) (struct) "KeepRelativeOffset" false 1.0 1.0 0.0 "/Game/Aanet/ovi.ovi" null)))))

(fn `UserConstructionScript`)